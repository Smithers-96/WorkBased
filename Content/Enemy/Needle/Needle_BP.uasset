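; Needle enemy that homes in on the player and deals contact damage.
; Tick moves its root toward the player's mesh using VInterpTo, without sweep.
; A capsule overlap with ThirdPersonCharacter halts it, and Tick subtracts clamped Health from the player through a DoOnce.
; A three-second Delay then restores speed, clears the hit flag and resets the DoOnce.
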(event OnComponentBeginOverlap(Capsule)
  (params (OverlappedComponent :type Primitive%20Component%20Object%20Reference) (OtherActor :type Actor%20Object%20Reference) (OtherComp :type Primitive%20Component%20Object%20Reference) (OtherBodyIndex :type Integer) (bFromSweep :type Boolean) (SweepResult :type Hit%20Result%20Structure%20%28by%20ref%29))
  (bind _asthird_person_character (Utilities|Casting|CastToThirdPersonCharacter OtherActor))
  (Variables|Default|SetPlayer _asthird_person_character)
  (Variables|Default|SetSpeed 0.0)
  (Variables|Default|Set?HitPlayer true))

(event Custom|MoveToPlayer
  ;[1 1 1] move to player
  (Transformation|SetWorldLocation (Variables|Default|GetDefaultSceneRoot) (Math|Interpolation|VInterpTo (Transformation|GetWorldLocation (Variables|Default|GetDefaultSceneRoot)) (Transformation|GetWorldLocation (Variables|/Script/Engine.Character|GetMesh (Game|GetPlayerCharacter 0))) (Variables|Default|GetDeltaSeconds) (Variables|Default|GetSpeed)) false false))

(event Custom|CanTakeDamage
  ;[1 1 1] when the Needle hits the player, stop moving for 2 seconds
  (Utilities|FlowControl|DoOnce false) ; enters at Reset
)

(event EventTick
  (params (DeltaSeconds :type Float%20%28single-precision%29))
  ;[1 1 1] when the Needle hits the player, stop moving for 2 seconds
  (if (Variables|Default|Get?HitPlayer)
    (Utilities|FlowControl|Sequence
      (:then_0
        (Utilities|FlowControl|DoOnce false
          (:Completed
            (CallFunction|DamagePlayer 0.2))))
      (:then_1
        (Utilities|FlowControl|Delay 3.0)
        (Variables|Default|SetSpeed 2.5)
        (Variables|Default|Set?HitPlayer false)
        (CallFunction|CanTakeDamage)))
    (else
      (Variables|Default|SetDeltaSeconds DeltaSeconds)
      (CallFunction|MovetoPlayer))))

(fn ConstructionScript)

(fn DamagePlayer
  (params (Value :type Float%20%28single-precision%29))
  (bind _asthird_person_character (Utilities|Casting|CastToThirdPersonCharacter (Game|GetPlayerCharacter 0))
    (:then
      (Variables|/Game/ThirdPersonBP/Blueprints/ThirdPersonCharacter.ThirdPersonCharacter_C|SetHealth _asthird_person_character (Math|Float|Clamp(Float) (- (Variables|/Game/ThirdPersonBP/Blueprints/ThirdPersonCharacter.ThirdPersonCharacter_C|GetHealth _asthird_person_character) Value)))
      (return))
    (:CastFailed
      (return))))