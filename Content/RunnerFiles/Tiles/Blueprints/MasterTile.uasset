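; Base floor tile for a runner game, which keeps the track going and speeds up the player as tiles are crossed.
; When the ThirdPersonCharacter overlaps its Box trigger, it calls SpawnTile on the ThirdPersonGameMode.
; It then raises player 0's max walk speed by a small clamped percentage and destroys itself after a short delay.
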(event OnComponentBeginOverlap(Box)
  (params (OverlappedComponent :type Primitive%20Component%20Object%20Reference) (OtherActor :type Actor%20Object%20Reference) (OtherComp :type Primitive%20Component%20Object%20Reference) (OtherBodyIndex :type Integer) (bFromSweep :type Boolean) (SweepResult :type Hit%20Result%20Structure%20%28by%20ref%29))
  ;[1 1 1] When the box collider, collides with the player, spawn the tile
  (Utilities|Casting|CastToThirdPersonCharacter OtherActor)
  (bind _asthird_person_game_mode (Utilities|Casting|CastToThirdPersonGameMode (Game|GetGameMode)))
  (Default|SpawnTile _asthird_person_game_mode)
  (bind _asthird_person_character (Utilities|Casting|CastToThirdPersonCharacter (Game|GetPlayerCharacter 0)))
  (Variables|/Script/Engine.CharacterMovementComponent|SetMaxWalkSpeed (Variables|/Script/Engine.Character|GetCharacterMovement _asthird_person_character) (Math|Float|Clamp(Float) (* (Variables|/Script/Engine.CharacterMovementComponent|GetMaxWalkSpeed (Variables|/Script/Engine.Character|GetCharacterMovement _asthird_person_character)) 1.01) 6e+02 1.2e+03))
  (Utilities|FlowControl|Delay 1.0)
  (Actor|DestroyActor) ; The tiles will destroy after the delay
)

(fn ConstructionScript)