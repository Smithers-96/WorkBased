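; Jump power-up pickup that temporarily doubles the ThirdPersonCharacter's jump velocity.
; On box overlap it casts to the character and, through a DoOnce that is never reset, plays a sound, prints a debug string and hides its mesh.
; After a five-second delay it restores a hardcoded default jump velocity; the actor is hidden rather than destroyed, so it works only once.
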(event OnComponentBeginOverlap(Box)
  (params (OverlappedComponent :type Primitive%20Component%20Object%20Reference) (OtherActor :type Actor%20Object%20Reference) (OtherComp :type Primitive%20Component%20Object%20Reference) (OtherBodyIndex :type Integer) (bFromSweep :type Boolean) (SweepResult :type Hit%20Result%20Structure%20%28by%20ref%29))
  (bind _asthird_person_character (Utilities|Casting|CastToThirdPersonCharacter OtherActor))
  (Utilities|FlowControl|DoOnce false
    (:Completed
      (Audio|PlaySound2D "/Game/Music/SoundCues/FX_power_up.FX_power_up")
      (Variables|/Script/Engine.CharacterMovementComponent|SetJumpZVelocity (Variables|/Script/Engine.Character|GetCharacterMovement _asthird_person_character) 1.2e+03) ; 600 is the player's standard jump height make it higher than 600 for the power up
      (Development|PrintString "JumpPowerUp")
      (Rendering|SetVisibility (Variables|Default|GetStaticMesh) false false)
      (Utilities|FlowControl|Delay 5.0 :!pinned true) ; Player's power up time
      (Variables|/Script/Engine.CharacterMovementComponent|SetJumpZVelocity (Variables|/Script/Engine.Character|GetCharacterMovement _asthird_person_character) 6e+02) ; This is the original jump height velocity
    )))

(fn ConstructionScript)